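; BP_P4Wall is a target wall for the fourth puzzle that shows a randomly chosen shape name and accepts the matching shape actor.
; Its Box overlap checks for sphere, cube, cylinder or cone puzzle actors, extracting the shape name by trimming the class display name.
; A match increments the referenced loop manager's iteration progress and blanks the target and text.
; Reset picks and displays a new random shape, as BeginPlay does.
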(event `self.ReceiveBeginPlay`
  (bind _output_get (set `self.TargetShape` (`KismetArrayLibrary.Array_Random` (`self.ShapeList`))))
  (`TextRenderComponent.K2_SetText` (`self.Shape_text`) (`KismetTextLibrary.Conv_StringToText` _output_get)))

(event `self.Box.OnComponentBeginOverlap`
  (params (OverlappedComponent :type "PrimitiveComponent Object Reference") (OtherActor :type "Actor Object Reference") (OtherComp :type "PrimitiveComponent Object Reference") (OtherBodyIndex :type Integer) (bFromSweep :type Boolean) (SweepResult :type "HitResult Structure (by ref)"))
  (bind _returnvalue (`GameplayStatics.GetObjectClass` OtherActor))
  (bind _returnvalue_2 (`KismetSystemLibrary.GetClassDisplayName` _returnvalue))
  (bind _output (`|ConvertAsset` (`self.LoopManagerinScene`)))
  (if (or (or (== _returnvalue "/Game/Blueprints/FourthPuzzle/BP_P4Sphere.BP_P4Sphere_C") (== _returnvalue "/Game/Blueprints/FourthPuzzle/BP_P4Cube.BP_P4Cube_C")) (or (== _returnvalue "/Game/Blueprints/FourthPuzzle/BP_P4Cylinder.BP_P4Cylinder_C") (== _returnvalue "/Game/Blueprints/FourthPuzzle/BP_P4Cone.BP_P4Cone_C")))
    (if (== (`KismetStringLibrary.GetSubstring` _returnvalue_2 5 (- (`KismetStringLibrary.Len` _returnvalue_2) 7)) (`self.TargetShape`))
      (set `/Game/Blueprints/TimeloopMechanic/BP_LoopManager.Progress in this iteration` (+ (`/Game/Blueprints/TimeloopMechanic/BP_LoopManager.Progress in this iteration` _output) 1) _output)
      (set `self.TargetShape` "")
      (`TextRenderComponent.K2_SetText` (`self.Shape_text`) ""))))

(fn `Reset`
  (bind _output_get (set `self.TargetShape` (`KismetArrayLibrary.Array_Random` (`self.ShapeList`))))
  (`TextRenderComponent.K2_SetText` (`self.Shape_text`) (`KismetTextLibrary.Conv_StringToText` _output_get)))

(fn `UserConstructionScript`)