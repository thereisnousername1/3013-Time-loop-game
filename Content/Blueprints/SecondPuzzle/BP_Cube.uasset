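; Interactable cube for the second puzzle that counts toward loop progress and relocates when used.
; A sphere trigger shows the hover message while the third-person character is inside it, and the construction script hides it initially.
; Interact increments the scene loop manager's progress for the current iteration, clears the cube's visibility flag, then moves it to the location from FindNewLocation if teleporting is allowed.
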(event `self.Sphere.OnComponentBeginOverlap`
  (params (OverlappedComponent :type "PrimitiveComponent Object Reference") (OtherActor :type "Actor Object Reference") (OtherComp :type "PrimitiveComponent Object Reference") (OtherBodyIndex :type Integer) (bFromSweep :type Boolean) (SweepResult :type "HitResult Structure (by ref)"))
  (bind _hover_message (`self.Hover Message`))
  ;[0.05127 0.05127 0.05127] Detect player enterance & exit
  (if (== (`GameplayStatics.GetObjectClass` OtherActor) "/Game/ThirdPerson/Blueprints/BP_ThirdPersonCharacter.BP_ThirdPersonCharacter_C")
    (`SceneComponent.SetVisibility` _hover_message true false)
    (`SceneComponent.SetHiddenInGame` _hover_message false false)))

(event `self.Sphere.OnComponentEndOverlap`
  (params (OverlappedComponent :type "PrimitiveComponent Object Reference") (OtherActor :type "Actor Object Reference") (OtherComp :type "PrimitiveComponent Object Reference") (OtherBodyIndex :type Integer))
  (bind _hover_message (`self.Hover Message`))
  ;[0.05127 0.05127 0.05127] Detect player enterance & exit
  (if (== (`GameplayStatics.GetObjectClass` OtherActor) "/Game/ThirdPerson/Blueprints/BP_ThirdPersonCharacter.BP_ThirdPersonCharacter_C")
    (`SceneComponent.SetVisibility` _hover_message false false)
    (`SceneComponent.SetHiddenInGame` _hover_message true false)))

(event `/Game/Blueprints/InteractInterface.Interact`
  (bind _output (`|ConvertAsset` (`self.Loop Managerin Scene`)))
  (set `/Game/Blueprints/TimeloopMechanic/BP_LoopManager.Progress in this iteration` (+ (`/Game/Blueprints/TimeloopMechanic/BP_LoopManager.Progress in this iteration` _output) 1) _output)
  (set `self.isVisible` false)
  (bind (_location _canteleport) (`self.FindNewLocation`))
  (if _canteleport
    (`self.K2_SetActorLocation` _location)))

(fn `UserConstructionScript`
  (`SceneComponent.SetVisibility` (`self.Hover Message`) false false))