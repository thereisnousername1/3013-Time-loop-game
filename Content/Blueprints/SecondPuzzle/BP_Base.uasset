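; Base actor for the second puzzle that teleports to another spot whenever the player stops seeing it.
; Tick uses WasRecentlyRendered to track visibility and triggers a single move on the change from rendered to unrendered.
; FindNewLocation draws random entries from the Locations actors, discarding any at its current position or flagged visible.
; If no candidate remains, the actor stays in place.
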(event `self.ReceiveTick`
  (params (DeltaSeconds :type "Float (single-precision)"))
  (if (`self.WasRecentlyRendered` 0.1)
    (set `self.isVisible` true)
    (elif (`self.isVisible`)
      (set `self.isVisible` false)
      (bind (_location _canteleport) (`self.FindNewLocation`))
      (if _canteleport
        (`self.K2_SetActorLocation` _location)))))

(fn `FindNewLocation`
  (returns (Location :type "Vector Structure") (CanTeleport :type Boolean))
  (locals (TempLocation :type "Array of /Game/Blueprints/SecondPuzzle/BP_SpawnLocation Object Reference") (CurrentIndex :type Integer :default 0))
  (bind _output_get (set `local.TempLocation` (`self.Locations`)))
  (bind _returnvalue (`KismetArrayLibrary.Array_Length` _output_get))
  (if (== _returnvalue 0) :!label _label
    (return (0.0 0.0 0.0) false)
    (else
      (set `local.CurrentIndex` (`KismetMathLibrary.RandomIntegerInRange` 0 (- _returnvalue 1)))
      (bind _output (`|GetArrayItem` _output_get (`local.CurrentIndex`)))
      (bind _returnvalue_2 (`self.K2_GetActorLocation` _output))
      (if (!= _returnvalue_2 (`self.K2_GetActorLocation`) :`ErrorTolerance` 5.0)
        (if (`/Game/Blueprints/SecondPuzzle/BP_SpawnLocation.isVisible` _output)
          _
          (else
            (return _returnvalue_2 true))))
      (`KismetArrayLibrary.Array_Remove` (`local.TempLocation`) (`local.CurrentIndex`))
      (goto _label))))

(fn `UserConstructionScript`)