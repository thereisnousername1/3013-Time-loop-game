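; BP_FirstPuzzle is an interactable actor that presents the first puzzle's question widget.
; Its sphere overlap shows a hover message while unscored and hides it on exit, without filtering by actor, as the character casts are unconnected.
; Interact creates W_Puzzle1 and shows the mouse cursor unless already open or scored.
; Otherwise it only hides the cursor and clears the open flag, leaving any widget in place.
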(event `self.Sphere.OnComponentBeginOverlap`
  (params (OverlappedComponent :type "PrimitiveComponent Object Reference") (OtherActor :type "Actor Object Reference") (OtherComp :type "PrimitiveComponent Object Reference") (OtherBodyIndex :type Integer) (bFromSweep :type Boolean) (SweepResult :type "HitResult Structure (by ref)"))
  (bind _hover_message (`self.Hover Message`))
  ;[0.05127 0.05127 0.05127] Detect player enterance & exit
  (if (`self.Scored`)
    (`SceneComponent.SetVisibility` _hover_message false false :!label _label)
    (else
      (`SceneComponent.SetVisibility` _hover_message true false))))

(event `self.Sphere.OnComponentEndOverlap`
  (params (OverlappedComponent :type "PrimitiveComponent Object Reference") (OtherActor :type "Actor Object Reference") (OtherComp :type "PrimitiveComponent Object Reference") (OtherBodyIndex :type Integer))
  ;[0.05127 0.05127 0.05127] Detect player enterance & exit
  (goto _label))

(event `/Game/Blueprints/InteractInterface.Interact`
  (bind _returnvalue (`GameplayStatics.GetPlayerController` 0))
  ;[0.05127 0.05127 0.05127] Puzzle 1 logic
  (if (`self.IsQuestionWidgetOpen`)
    (bind _output_get (set `PlayerController.bShowMouseCursor` false _returnvalue :!label _label_2))
    (set `self.IsQuestionWidgetOpen` _output_get)
    (elif (`self.Scored`)
      (goto _label_2)
      (else
        (bind _returnvalue_2 (`|CreateWidget` "/Game/Blueprints/FirstPuzzle/W_Puzzle1.W_Puzzle1_C" _returnvalue))
        (`UserWidget.AddToViewport` _returnvalue_2 0)
        (bind _output_get_2 (set `PlayerController.bShowMouseCursor` true _returnvalue))
        (set `self.IsQuestionWidgetOpen` _output_get_2)))))

(fn `UserConstructionScript`)