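; Manager for the timeloop mechanic: when the timer reaches the limit, it judges puzzle progress and returns the player to the start.
; Tick advances the timer and its UI string, then calls ResetGame on expiry.
; Enough progress within allowed attempts resets puzzles, raises the requirement up to a cap and shortens the limit; otherwise an attempt is used.
; Running out of attempts opens the lose level, while enough successful loops opens the win level.
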(event `self.ReceiveBeginPlay`
  (set `self.Current Time` 0.0)
  (set `self.Progress in this iteration` 0)
  (set `self.Current Attempt` 1))

(event `self.ReceiveTick`
  (params (DeltaSeconds :type "Float (single-precision)"))
  (`self.Timer`)
  (set `self.Progress in this iteration` (`self.Progress in this iteration`))
  (set `self.Current Attempt` (`self.Current Attempt`)))

(event `Timer`
  (bind _output_get (set `self.Current Time` (+ (`self.Current Time`) (`GameplayStatics.GetWorldDeltaSeconds`))))
  (set `self.TimeToString` (`KismetStringLibrary.TimeSecondsToString` _output_get)) ; To the timer in UI
  (if (>= (`self.Current Time`) (`self.Time Limit`))
    (`self.ResetGame`)))

(fn `ResetGame`
  (bind _returnvalue (`GameplayStatics.GetPlayerController` 0))
  (bind _progress_needed (`self.Progress needed`))
  (bind _playerstart (`self.PlayerStart`))
  (if (and (>= (`self.Progress in this iteration`) (`self.Progress needed`)) (<= (`self.Current Attempt`) (`self.Max Attempts`)))
    (set `self.Current Time` 0.0)
    (set `self.Total Progress` (+ (`self.Total Progress`) 1))
    (if (>= _progress_needed 6)
      (set `self.Progress needed` 6)
      (else
        (set `self.Progress needed` (+ _progress_needed 1))))
    (bind _output_get (set `self.Time Limit` (- (`self.Time Limit`) (`self.(For debug use)Decrement time`))))
    (set `/Game/Blueprints/FirstPuzzle/BP_FirstPuzzle.Scored` false (`|ConvertAsset` (`self.Puzzle1`)))
    (set `/Game/Blueprints/SixthPuzzle/BP_SixthPuzzle.Scored` false (`|ConvertAsset` (`self.Puzzle6`)))
    (set `self.Progress in this iteration` 0)
    ;[0.05127 0.05127 0.05127] Third Puzzle Reset
    (for _array_element (`self.ThirdPuzzle_Array`)
      (set `/Game/Blueprints/ThirdPuzzle/BP_pod.isOn` false _array_element)
      (`/Game/Blueprints/FourthPuzzle/BP_P4Wall.Reset` (`|ConvertAsset` (`self.Puzzle4`)))
      (`/Game/Blueprints/FifthPuzzle/BP_P5Wall.Reset` (`|ConvertAsset` (`self.Puzzle5`)))
      ;[0.05127 0.05127 0.05127] Reset Player
      (`GameModeBase.RestartPlayerAtPlayerStart` (`GameplayStatics.GetGameMode`) _returnvalue _playerstart :!label _label)
      (`self.K2_SetActorLocationAndRotation` (`GameplayStatics.GetPlayerCharacter` 0) (`self.K2_GetActorLocation` _playerstart) (`self.K2_GetActorRotation` _returnvalue) false false)
      ;[0.05127 0.05127 0.05127] Simple Losing Condition
      (if (>= (`self.Current Attempt`) (`self.Max Attempts`))
        (`GameplayStatics.OpenLevelBySoftObjectPtr` "/Game/Scene/LoseEnding.LoseEnding")
        (else
          ;[0.05127 0.05127 0.05127] Simple Winning Condition Checking
          (if (>= (`self.Total Progress`) (`self.Total iterations`))
            (`GameplayStatics.OpenLevelBySoftObjectPtr` "/Game/Scene/WinEnding.WinEnding")))))
    (else
      (set `self.Current Time` 0.0)
      (set `self.Current Attempt` (+ (`self.Current Attempt`) 1))
      (goto _label))))

(fn `UserConstructionScript`)