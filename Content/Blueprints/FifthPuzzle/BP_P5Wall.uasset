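; BP_P5Wall is a fifth-puzzle wall that displays a randomly chosen material name and scores when a matching actor enters its Box.
; BeginPlay and Reset pick the target from MaterialArray and show its name without the two-character prefix.
; Overlaps compare that text to a substring of the actor's object name, so matching depends on naming conventions.
; A match increments the loop manager's iteration progress and clears the target and text.
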(event `self.ReceiveBeginPlay`
  (bind _output_get (set `self.TargetMat` (`KismetArrayLibrary.Array_Random` (`self.MaterialArray`))))
  (bind _returnvalue (`KismetSystemLibrary.GetDisplayName` _output_get))
  (`TextRenderComponent.K2_SetText` (`self.Material_text`) (`KismetTextLibrary.Conv_StringToText` (`KismetStringLibrary.GetSubstring` _returnvalue 2 (- (`KismetStringLibrary.Len` _returnvalue) 2)))))

(event `self.Box.OnComponentBeginOverlap`
  (params (OverlappedComponent :type "PrimitiveComponent Object Reference") (OtherActor :type "Actor Object Reference") (OtherComp :type "PrimitiveComponent Object Reference") (OtherBodyIndex :type Integer) (bFromSweep :type Boolean) (SweepResult :type "HitResult Structure (by ref)"))
  (bind _returnvalue (`KismetSystemLibrary.GetObjectName` OtherActor))
  (bind _returnvalue_2 (`KismetSystemLibrary.GetDisplayName` (`self.TargetMat`)))
  (bind _output (`|ConvertAsset` (`self.LoopManagerinScene`)))
  (if true
    (if (== (`KismetTextLibrary.Conv_StringToText` (`KismetStringLibrary.GetSubstring` _returnvalue 5 (- (`KismetStringLibrary.Len` _returnvalue) 9))) (`KismetTextLibrary.Conv_StringToText` (`KismetStringLibrary.GetSubstring` _returnvalue_2 2 (- (`KismetStringLibrary.Len` _returnvalue_2) 2))))
      (set `/Game/Blueprints/TimeloopMechanic/BP_LoopManager.Progress in this iteration` (+ (`/Game/Blueprints/TimeloopMechanic/BP_LoopManager.Progress in this iteration` _output) 1) _output)
      (set `self.TargetMat` null)
      (`TextRenderComponent.K2_SetText` (`self.Material_text`) ""))))

(fn `Reset`
  (bind _output_get (set `self.TargetMat` (`KismetArrayLibrary.Array_Random` (`self.MaterialArray`))))
  (bind _returnvalue (`KismetSystemLibrary.GetDisplayName` _output_get))
  (`TextRenderComponent.K2_SetText` (`self.Material_text`) (`KismetTextLibrary.Conv_StringToText` (`KismetStringLibrary.GetSubstring` _returnvalue 2 (- (`KismetStringLibrary.Len` _returnvalue) 2)))))

(fn `UserConstructionScript`)