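; BP_base is the base actor for the third puzzle, detecting when it is solved and crediting loop progress.
; Each Tick it checks whether all nine Scoring elements are on.
; When they are, it increments ProgressInThisIteration on the scene's loop manager, then switches every element off to reset the puzzle.
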(event `self.ReceiveTick`
  (params (DeltaSeconds :type "Float (single-precision)"))
  (bind _scoring (`self.Scoring`))
  (bind _output (`|ConvertAsset` (`self.Loop Managerin Scene`)))
  (if (and (== (`/Game/Blueprints/ThirdPuzzle/BP_pod.isOn` (`|GetArrayItem` _scoring)) true) (== (`/Game/Blueprints/ThirdPuzzle/BP_pod.isOn` (`|GetArrayItem` _scoring 1)) true) (== (`/Game/Blueprints/ThirdPuzzle/BP_pod.isOn` (`|GetArrayItem` _scoring 2)) true) (== (`/Game/Blueprints/ThirdPuzzle/BP_pod.isOn` (`|GetArrayItem` _scoring 3)) true) (== (`/Game/Blueprints/ThirdPuzzle/BP_pod.isOn` (`|GetArrayItem` _scoring 4)) true) (== (`/Game/Blueprints/ThirdPuzzle/BP_pod.isOn` (`|GetArrayItem` _scoring 5)) true) (== (`/Game/Blueprints/ThirdPuzzle/BP_pod.isOn` (`|GetArrayItem` _scoring 6)) true) (== (`/Game/Blueprints/ThirdPuzzle/BP_pod.isOn` (`|GetArrayItem` _scoring 7)) true) (== (`/Game/Blueprints/ThirdPuzzle/BP_pod.isOn` (`|GetArrayItem` _scoring 8)) true))
    (set `/Game/Blueprints/TimeloopMechanic/BP_LoopManager.Progress in this iteration` (+ (`/Game/Blueprints/TimeloopMechanic/BP_LoopManager.Progress in this iteration` _output) 1) _output)
    ;[0.05127 0.05127 0.05127] Third Puzzle Reset
    (for _array_element (`self.Scoring`)
      (set `/Game/Blueprints/ThirdPuzzle/BP_pod.isOn` false _array_element))))

(fn `UserConstructionScript`)