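; BP_SixthPuzzle is an interactable puzzle actor that shows a randomly chosen question widget for the game's sixth puzzle.
; Its sphere overlap events show and hide a hover message for any actor, as the character casts are unconnected.
; Interact creates a random widget from QuestionArray and shows the mouse cursor, tracking this with IsQuestionWidgetOpen.
; Interacting again hides the cursor and clears that flag without removing the widget.
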(event `self.Sphere.OnComponentBeginOverlap`
  (params (OverlappedComponent :type "PrimitiveComponent Object Reference") (OtherActor :type "Actor Object Reference") (OtherComp :type "PrimitiveComponent Object Reference") (OtherBodyIndex :type Integer) (bFromSweep :type Boolean) (SweepResult :type "HitResult Structure (by ref)"))
  ;[0.05127 0.05127 0.05127] Detect player enterance & exit
  (`SceneComponent.SetVisibility` (`self.Hover Message`) true false))

(event `self.Sphere.OnComponentEndOverlap`
  (params (OverlappedComponent :type "PrimitiveComponent Object Reference") (OtherActor :type "Actor Object Reference") (OtherComp :type "PrimitiveComponent Object Reference") (OtherBodyIndex :type Integer))
  ;[0.05127 0.05127 0.05127] Detect player enterance & exit
  (`SceneComponent.SetVisibility` (`self.Hover Message`) false false))

(event `self.Interact`
  (bind _returnvalue (`GameplayStatics.GetPlayerController` 0))
  ;[0.05127 0.05127 0.05127] Puzzle 6 logic
  (if (`self.IsQuestionWidgetOpen`)
    (bind _output_get (set `PlayerController.bShowMouseCursor` false _returnvalue))
    (set `self.IsQuestionWidgetOpen` _output_get)
    (else
      (bind _returnvalue_2 (`|CreateWidget` (`KismetArrayLibrary.Array_Random` (`self.QuestionArray`)) _returnvalue))
      (`UserWidget.AddToViewport` _returnvalue_2 0)
      (bind _output_get_2 (set `PlayerController.bShowMouseCursor` true _returnvalue))
      (set `self.IsQuestionWidgetOpen` _output_get_2))))

(fn `UserConstructionScript`)